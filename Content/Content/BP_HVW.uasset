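; BP_HVW is a child character Blueprint that adds forward and backward shooting input on top of inherited movement and aiming.
; PrimaryAttack sets ShootType to forward or backward depending on whether AimAction is held at press time, and clears it on release.
; The BPI_Get_EssentialValues override passes the parent's locomotion values through and supplies its own forward and backward shooting flags, which no graph here sets.
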(event EventBeginPlay)

(event Collision|EventActorBeginOverlap
  (params (OtherActor :type Actor%20Object%20Reference)))

(event EventTick
  (params (DeltaSeconds :type Float%20%28single-precision%29)))

(event Input|ActionEvents|InputActionPrimaryAttack
  (params (Key :type Key%20Structure :default "None"))
  (:Pressed
    (if (Variables|Default|GetIs%20Being%20Backward%20Aiming)
      (switch Utilities|FlowControl|Switch|SwitchonH_ShootType (Variables|Default|GetShootType)
        (:NewEnumerator2
          _)
        (:NewEnumerator1
          _))
      (Variables|Default|SetShootType "NewEnumerator0")
      (else
        (switch Utilities|FlowControl|Switch|SwitchonH_ShootType (Variables|Default|GetShootType)
          (:NewEnumerator2
            _)
          (:NewEnumerator0
            _))
        (Variables|Default|SetShootType "NewEnumerator1"))))
  (:Released
    (Variables|Default|SetShootType "NewEnumerator2")))

(event Input|ActionEvents|InputActionAimAction
  (params (Key :type Key%20Structure :default "None"))
  (:Pressed
    (Variables|Default|SetIs%20Being%20Backward%20Aiming true))
  (:Released
    (Variables|Default|SetIs%20Being%20Backward%20Aiming false)))

(fn ConstructionScript)

(fn BPIGetEssentialValues
  (bind (_acceleration _movement_input_ace _velocity _speed _movement_input_amount _aiming_rotator _aim_yaw_rotate_rate _ismoving _hasmovementinput) (|CallParentFunction))
  (return _acceleration _movement_input_ace _velocity _speed _movement_input_amount _aiming_rotator _aim_yaw_rotate_rate _ismoving _hasmovementinput (Variables|Default|GetIs%20Being%20Forward%20S) (Variables|Default|GetIs%20Backward%20S)))