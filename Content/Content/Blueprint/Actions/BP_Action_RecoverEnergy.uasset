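; Action Blueprint that restores the owning player character's energy to its initial level after a short delay.
; Starting the action sets a one-shot timer, whose callback casts the owner to HPlayerCharacter and calls RestoreEnergyToInitLevel on its attribute component.
; Stopping the action clears the timer, cancelling any pending recovery.
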(event Custom|RecoverEnergy
  (bind _ashplayer_character (Utilities|Casting|CastToHPlayerCharacter (Components|GetOwner (Class|HAction|GetOwningComponent))))
  (Class|HAttributeComponent|RestoreEnergytoInitLevel (Actor|GetComponentbyClass _ashplayer_character "/Script/HDZMSandbox.HAttributeComponent")))

(event EventStartAction
  (params (Instigator :type Actor%20Object%20Reference))
  (|CallParentFunction Instigator)
  (bind _returnvalue (Utilities|Time|SetTimerbyEvent (delegate Custom|RecoverEnergy) 3.0))
  (Variables|Default|SetTimerHandle_RevoerEnergy _returnvalue))

(event EventStopAction
  (params (Instigator :type Actor%20Object%20Reference))
  (|CallParentFunction Instigator)
  (Utilities|Time|ClearandInvalidateTimerbyHandle (Variables|Default|GetTimerHandle_RevoerEnergy)))