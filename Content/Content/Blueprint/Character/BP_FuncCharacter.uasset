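; Child character Blueprint that adds forward and backward shooting state on top of a parent character with locomotion-state interfaces.
; Holding AimAction flags backward aiming and switches rotation mode, restoring the desired mode on release.
; PrimaryAttack sets ShootType to backward or forward based on that flag, and clears it on release.
; The current-state interface override passes parent values through and adds ShootType, while the essential-values override only forwards the parent's.
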(event EventBeginPlay)

(event Collision|EventActorBeginOverlap
  (params (OtherActor :type Actor%20Object%20Reference)))

(event Input|ActionEvents|InputActionPrimaryAttack
  (params (Key :type Key%20Structure))
  ;[1 1 1] Input: Shoot
  (:Pressed
    (if (Variables|Default|GetIs%20Being%20Backward%20Aiming)
      (switch Utilities|FlowControl|Switch|SwitchonH_ShootType (Variables|Default|GetShootType)
        (:NewEnumerator1
          _)
        (:NewEnumerator2
          _))
      (Variables|Default|SetShootType "NewEnumerator0")
      (else
        (switch Utilities|FlowControl|Switch|SwitchonH_ShootType (Variables|Default|GetShootType)
          (:NewEnumerator0
            _)
          (:NewEnumerator2
            _))
        (Variables|Default|SetShootType "NewEnumerator1"))))
  (:Released
    (Variables|Default|SetShootType "NewEnumerator2")))

(event Input|ActionEvents|InputActionAimAction
  (params (Key :type Key%20Structure))
  ;[1 1 1] Input Aiming. 注意, 父类的响应也会被调用
  (:Pressed
    (Variables|Default|SetIs%20Being%20Backward%20Aiming true)
    (CallFunction|BPISetRotationMode "NewEnumerator2"))
  (:Released
    (Variables|Default|SetIs%20Being%20Backward%20Aiming false)
    (CallFunction|BPISetRotationMode (Variables|Default|GetDesired%20RotationMode))))

(event EventTick
  (params (DeltaSeconds :type Float%20%28single-precision%29)))

(fn ConstructionScript)

(fn BPIGetEssentialValues
  (bind (_acceleration _movement_input_ace _velocity _speed _movement_input_amount _aiming_rotator _aim_yaw_rotate_rate _ismoving _hasmovementinput) (|CallParentFunction))
  (return _acceleration _movement_input_ace _velocity _speed _movement_input_amount _aiming_rotator _aim_yaw_rotate_rate _ismoving _hasmovementinput))

(fn BPIGetCurrentState
  (bind (_pawnmovementmode _movementstate _prevmovementstate _movement_action _rotationmode _actual_gait _actual_stance _view_mode _overlay_state) (|CallParentFunction))
  (return _pawnmovementmode _movementstate _prevmovementstate _movement_action _rotationmode _actual_gait _actual_stance _view_mode _overlay_state (Variables|Default|GetShootType)))