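; Game mode Blueprint that spawns a shared InfoProvider and respawns killed players.
; BeginPlay spawns and stores the InfoProvider, which BPIGetInfoProvider returns when valid.
; OnPlayerKilledReBorn starts a one-second timer, after which the dead pawn's controller unpossesses and is restarted through RestartPlayer.
; If that pawn has no PlayerController, an error about a wrongly tagged non-player is printed instead.
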(event Custom|OnPlayerKilledReBorn
  (params (PlayerC :type H%20Player%20Character%20Object%20Reference))
  (Utilities|Time|SetTimerbyEvent (delegate Custom|OnPlayerKilled) 1.0))

(event Custom|OnPlayerKilled
  (bind _asplayer_controller (Utilities|Casting|CastToPlayerController (Pawn|GetController (stale Custom|OnPlayerKilledReBorn PlayerC)))
    (:then
      (CallFunction|RespawnPlayElaps _asplayer_controller))
    (:CastFailed
      (Development|PrintString "error Tag:an nonPlayer without playercontroller  has the Player tag " true true "(R=1.000000,G=0.058872,B=0.000000,A=1.000000)"))))

(event EventBeginPlay
  (bind _returnvalue (Game|SpawnActorfromClass "/Game/Content/Blueprint/STG/System/InfoProvider.InfoProvider_C" (Math|Transform|MakeTransform "0, 0, 0" "0, 0, 0" "1,1,1") "Undefined" 0 0))
  (Variables|Default|SetTemp%20InfoProvide _returnvalue))

(event EventTick
  (params (DeltaSeconds :type Float%20%28single-precision%29)))

(fn ConstructionScript)

(fn RespawnPlayElaps
  (params (Controller :type Player%20Controller%20Object%20Reference))
  (Utilities|IsValid Controller
    (:Is%20Valid
      (Pawn|UnPossess Controller)
      (Class|GameModeBase|RestartPlayer Controller))))

(fn BPIGetInfoProvider
  (bind _temp_infoprovide (Variables|Default|GetTemp%20InfoProvide))
  (Utilities|IsValid _temp_infoprovide
    (:Is%20Valid
      (return _temp_infoprovide))))