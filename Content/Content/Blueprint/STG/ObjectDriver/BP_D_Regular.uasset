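; BP_D_Regular is an object driver for the STG system that moves its owner with constant linear and yaw acceleration.
; Each DriverUpdate integrates both velocities, then applies a local transform along the owner's forward X axis and around yaw, so a turn rate curves the path.
; Interface events and getters expose the four motion values, and CloneOne copies them onto the duplicate created by the parent.
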(event EventDriverUpdate
  (params (DeltaTime :type Float%20%28single-precision%29))
  (|CallParentFunction DeltaTime)
  (bind _output_get (Variables|Default|SetLinearV (+ (Variables|Default|GetLinearV) (* DeltaTime (Variables|Default|GetLinearA)))))
  (bind _output_get_2 (Variables|Default|SetRotV (+ (Variables|Default|GetRotV) (* DeltaTime (Variables|Default|GetRotA)))))
  (Class|Actor|AddActorLocalTransform (Variables|Default|GetOwninger) (Math|Transform|MakeTransform (* "1.000000, 0, 0" (* _output_get DeltaTime)) (Math|Rotator|MakeRotator 0.0 0.0 (* _output_get_2 DeltaTime)) "1,1,1") false false))

(event EventBPISetLinearVelocity
  (params (LV :type Float%20%28single-precision%29))
  (Variables|Default|SetLinearV LV))

(event EventBPISetLinearAcceleration
  (params (LA :type Float%20%28single-precision%29))
  (Variables|Default|SetLinearA LA))

(event EventBPISetRotVelocity
  (params (RV :type Float%20%28single-precision%29))
  (Variables|Default|SetRotV RV))

(event EventBPISetRotAcceleration
  (params (RA :type Float%20%28single-precision%29))
  (Variables|Default|SetRotA RA))

(fn InitRegular)

(fn CloneOne
  (bind _returnvalue (|CallParentFunction))
  (bind _asbp_d_regular (Utilities|Casting|CastToBP_D_Regular _returnvalue)
    (:then
      (Variables|BP_D_Regular_C|SetLinearV _asbp_d_regular (Variables|Default|GetLinearV))
      (Variables|BP_D_Regular_C|SetLinearA _asbp_d_regular (Variables|Default|GetLinearA))
      (Variables|BP_D_Regular_C|SetRotV _asbp_d_regular (Variables|Default|GetRotV))
      (Variables|BP_D_Regular_C|SetRotA _asbp_d_regular (Variables|Default|GetRotA))
      (return _asbp_d_regular))
    (:CastFailed
      (Development|PrintString 0 "Test Faild"))))

(fn BPIGetLinearAcceleration
  (return (Variables|Default|GetLinearA)))

(fn BPIGetLinearVelocity
  (return (Variables|Default|GetLinearV)))

(fn BPIGetRotAcceleration
  (return (Variables|Default|GetRotA)))

(fn BPIGetRotVelocity
  (return (Variables|Default|GetRotV)))