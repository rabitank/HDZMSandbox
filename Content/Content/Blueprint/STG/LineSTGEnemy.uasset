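; Bullet-hell enemy that fires patterned bullets by cloning a prototype bullet configured at init.
; Init also builds arc and UV-sphere position generators and fetches an info provider from the game mode.
; After a short delay, BeginPlay runs stage 2, which spawns an attached BP_SP_PGGen pattern spawner and opens its senders.
; Timeline-driven stage 1, firing player-aimed sphere and arc patterns, is present but its call is disconnected.
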(event Custom|OnInit
  (bind _returnvalue (Transformation|GetActorLocation))
  (bind _returnvalue_2 (Transformation|GetActorRotation))
  ;[1 1 1] Init
  (Utilities|FlowControl|Sequence
    (:then_0
      ;;[1 1 1] Sample Bullet
      (bind _returnvalue_3 (Game|SpawnActorfromClass "/Game/Content/Blueprint/STG/STGBullet/BP_MB_TestWithArgument.BP_MB_TestWithArgument_C" (Math|Transform|MakeTransform "0, 0, 0" "0, 0, 0" "1,1,1") "AlwaysSpawn" self 0))
      (Class|RegularMoveBPI|BPISetLinearVelocity(Message) (Class|HComplexBullet|GetDriverRef _returnvalue_3) 8e+02)
      (Class|HBulletBase|PrototypingYXH _returnvalue_3)
      (Class|HBulletBase|ResetFadeTime _returnvalue_3 4.0) ; this time is for clonedObj
      (Variables|Default|SetSampleBullet _returnvalue_3))
    (:then_1
      (bind _returnvalue_4 (Game|ConstructObjectfromClass "/Game/Content/Blueprint/STG/placementGenerator/BP_PG_arc.BP_PG_arc_C" self))
      (bind _output_get (Variables|Default|SetStage1_PG1_arc _returnvalue_4))
      (Default|Reset _output_get _returnvalue _returnvalue_2 3.6e+02 (Variables|ShootControl|GetNum%20Pre%20Line) 0.0 2e+02)
      (EventDispatchers|BindEventtoPGCompleted _output_get (EventDispatchers|CreateEvent :!event Custom|OnPGComleted))
      (bind _returnvalue_5 (Game|ConstructObjectfromClass "/Game/Content/Blueprint/STG/placementGenerator/BP_PG_UVSphere.BP_PG_UVSphere_C" self))
      (Default|ResetPG _returnvalue_5 _returnvalue _returnvalue_2 9e+01 1.8e+02 10 15 1e+02 0.0 false)
      (EventDispatchers|BindEventtoPGCompleted _returnvalue_5 (EventDispatchers|CreateEvent :!event Custom|OnPGComleted))
      (Variables|Default|SetStage1_PG2_uvsphere _returnvalue_5))
    (:then_2
      (bind _provider (Class|STGSystemBPI|BPIGetInfoProvider(Message) (Game|GetGameMode)))
      (Variables|Default|SetProvider _provider))
    (:then_3
      (bind _returnvalue_6 (Game|ConstructObjectfromClass "/Game/Content/Blueprint/STG/ObjectDriver/BP_D_Regular.BP_D_Regular_C" self))
      (Class|HDriver|CloneOne _returnvalue_6))))

(event Custom|ShootStage1
  (bind _stage1_pg1_arc (Variables|Default|GetStage1_PG1_arc))
  (bind _stage1_pg2_uvsphere (Variables|Default|GetStage1_PG2_uvsphere))
  (bind _stage1_pg1_arc_2 (Variables|Default|GetStage1_PG1_arc))
  (bind _samplebullet (Variables|Default|GetSampleBullet))
  (bind _returnvalue (Class|HComplexBullet|GetDriverRef _samplebullet))
  ;[1 1 1] Stage1
  (Variables|/Game/Content/Blueprint/STG/placementGenerator/BP_PG_UVSphere.BP_PG_UVSphere_C|SetIsdiffuse (Variables|Default|GetStage1_PG2_uvsphere) false)
  (bind (_direction _timespeed _yawrange _bulletspeedfactor) (Timeline|ChooseTy Play)
    (:Update
      ;;[1 1 1] 累积计时
      (bind _output_get (Variables|Default|SetIntervalTime (+ (* (+ _timespeed 1.0) (Utilities|Time|GetWorldDeltaSeconds)) (Variables|Default|GetIntervalTime))))
      (if (>= _output_get (Variables|Default|GetCurIntreval))
        (Utilities|FlowControl|Sequence
          (:then_0
            ;;[1 1 1] 配置子弹原型
            (bind _lv (Class|RegularMoveBPI|BPIGetLinearVelocity(Message) _returnvalue))
            (Variables|Default|SetIntervalTime 0.0)
            (Class|RegularMoveBPI|BPISetLinearVelocity(Message) _returnvalue (* _lv _bulletspeedfactor)))
          (:then_1
            ;;[1 1 1] 配置位置生成器
            (Default|SetRollAngle _stage1_pg2_uvsphere (* _yawrange 1.8e+02))
            (Default|SetDirection _stage1_pg2_uvsphere (Default|GetPlayerDirection (Variables|Default|GetProvider) (Transformation|GetActorLocation)))
            (CallFunction|PGOnceShoot (Variables|Default|GetSampleBullet) (Variables|Default|GetStage1_PG2_uvsphere)) ; a PG's adapter, 在叶子类中的包装函数,高度特化,不用考虑给其他人复用. 或者你可以考虑搞个包装类复用?
          ))))
    (:Finished
      (Variables|/Game/Content/Blueprint/STG/placementGenerator/BP_PGBase.BP_PGBase_C|SetDirectionYawOffset _stage1_pg1_arc 8e+01)
      (Default|SetRadius _stage1_pg1_arc 3e+02)
      (bind _timespeed_2 (Timeline|Timeline_0 Play)
        (:Update
          ;;[1 1 1] 累积计时
          (bind _output_get_2 (Variables|Default|SetIntervalTime (+ (* (+ _timespeed_2 1.0) (Utilities|Time|GetWorldDeltaSeconds)) (Variables|Default|GetIntervalTime))))
          (if (>= _output_get_2 (Variables|Default|GetCurSingalShootInterval))
            (Variables|/Game/Content/Blueprint/STG/placementGenerator/BP_PGBase.BP_PGBase_C|SetCentDirect _stage1_pg1_arc_2 (Default|GetPlayerDirection (Variables|Default|GetProvider) (Transformation|GetActorLocation)))
            (bind (_pos _direction_2) (Default|Pop _stage1_pg1_arc_2))
            (Class|HBulletBase|Cloneto (Variables|Default|GetSampleBullet) _pos _direction_2)))))))

(event Custom|ShootStage2
  (bind _returnvalue (Game|SpawnActorfromClass "/Game/Content/Blueprint/STG/SenderSystem/SenderPattern/BP_SP_PGGen.BP_SP_PGGen_C" (Transformation|GetActorTransform) "AlwaysSpawn" 0 self))
  (bind _output_get (Variables|Default|SetSP _returnvalue))
  (Class|HSenderPattern|InitPattern _output_get 0.5 (Variables|Default|GetSampleBullet))
  (Transformation|AttachActorToActor _output_get self "None" "KeepWorld" "KeepWorld" "KeepWorld" true)
  (Class|HSenderPattern|OpenSenders (Variables|Default|GetSP)))

(event Custom|OnPGComleted
  (bind _stage1_pg2_uvsphere (Variables|Default|GetStage1_PG2_uvsphere))
  (bind _timeline_0 (Variables|Default|GetTimeline_0))
  ;[1 1 1] Stage1
  (if (Audio|Components|Audio|IsPlaying _timeline_0)
    (Audio|Components|Audio|Stop _timeline_0)
    (Default|ResetPG _stage1_pg2_uvsphere (Transformation|GetActorLocation) "0, 0, 0" 3.6e+02 1.8e+02 20 10 8e+01 0.0 true)
    (CallFunction|PGOnceShoot (Variables|Default|GetSampleBullet) _stage1_pg2_uvsphere)
    (Utilities|FlowControl|Delay 2.0)
    (CallFunction|ShootStage2)))

(event EventBeginPlay
  ;[1 1 1] Line
  (CallFunction|OnInit)
  (Utilities|FlowControl|Delay 2.0)
  (CallFunction|ShootStage2))

(event Collision|EventActorBeginOverlap
  (params (OtherActor :type Actor%20Object%20Reference))
  ;[1 1 1] Init
)

(event EventTick
  (params (DeltaSeconds :type Float%20%28single-precision%29))
  ;[1 1 1] Stage1
)

(fn ConstructionScript)

(fn PGOnceShoot
  (params (BulletIns :type H%20Bullet%20Base%20Object%20Reference) (PG :type BP%20PG%20Base%20Object%20Reference))
  (Utilities|IsValid BulletIns
    (:Is%20Valid
      (LocalVariables|SetNum (Variables|/Game/Content/Blueprint/STG/placementGenerator/BP_PGBase.BP_PGBase_C|GetNum PG))
      (LocalVariables|SetYaw%20Stride (/ 0.0 (Math|Conversions|ToFloat(Integer) (LocalVariables|Getnum))))
      (for _index (range 0 (- (LocalVariables|Getnum) 1))
        (bind (_pos _direction) (Default|Pop PG))
        (Class|HBulletBase|Cloneto BulletIns _pos _direction)))))