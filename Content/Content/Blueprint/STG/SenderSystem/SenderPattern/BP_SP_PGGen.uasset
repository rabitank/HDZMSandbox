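; BP_SP_PGGen is a sender pattern for the STG bullet system that lays out its senders using a point generator.
; Its SetSendersInitData override constructs a BP_PG_arc, configures it with a center direction, count and radius, then pops each point's position and direction into the parent's sender list.
; Each popped position is also printed for debugging, and InitPattern only forwards to the parent.
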(event EventBeginPlay)

(event Collision|EventActorBeginOverlap
  (params (OtherActor :type Actor%20Object%20Reference)))

(event EventTick
  (params (DeltaSeconds :type Float%20%28single-precision%29)))

(event EventInitPattern
  (params (interval :type Float%20%28single-precision%29) (samplebulle :type H%20Bullet%20Base%20Object%20Reference))
  (|CallParentFunction interval samplebulle))

(fn ConstructionScript)

(fn SetSendersInitData
  (bind _datas (|CallParentFunction))
  (bind _returnvalue (Game|ConstructObjectfromClass "/Game/Content/Blueprint/STG/placementGenerator/BP_PG_arc.BP_PG_arc_C" self))
  (bind _output_get (Variables|Default|SetPG _returnvalue))
  (Default|Reset _output_get "0, 0, 0" "90.000000,180.000000,0.000000" 1.2e+02 16 0.0 2e+02)
  (for _index (range 0 15)
    (bind (_pos _direction) (Default|Pop (Variables|Default|GetPG)))
    (Development|PrintString (Utilities|String|ToString(Vector) _pos))
    (Utilities|Array|Add _datas (Utilities|Struct|MakeSenderInitData _pos _direction 0)))
  (return _datas))