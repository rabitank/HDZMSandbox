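; Straight-line bullet actor for an STG (shoot 'em up) mode that travels briefly, halts, then expands in a "Boom" effect.
; On BeginPlay, a looping timer steps it along local X without sweeping, while a one-shot timer later clears that movement.
; After a short pause, the Boom timeline drives a uniform scale-up.
; The graph contains no overlap handling, damage or destroy logic.
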(event Custom|OnInit
  (Utilities|Time|SetTimerbyEvent (delegate Custom|endMove) 1.0)
  (bind _returnvalue (Utilities|Time|SetTimerbyEvent (delegate Custom|shoot1) 0.1 true 0.2))
  (Variables|Default|SetMoveHandle _returnvalue))

(event Custom|shoot1
  (Transformation|AddActorLocalOffset "5.000000, 0, 0" false false))

(event Custom|endMove
  (Utilities|Time|ClearandInvalidateTimerbyHandle (Variables|Default|GetMoveHandle))
  (Utilities|Time|SetTimerbyEvent (delegate Custom|OnEndMove) 0.4))

(event Custom|OnEndMove
  (bind _scale (Timeline|boom Play)
    (:Update
      (Transformation|SetActorRelativeScale3D (Math|Conversions|ToVector(Float) (+ _scale 1.0))))))

(event EventBeginPlay
  (CallFunction|OnInit))

(event Collision|EventActorBeginOverlap
  (params (OtherActor :type Actor%20Object%20Reference)))

(event EventTick
  (params (DeltaSeconds :type Float%20%28single-precision%29)))

(fn ConstructionScript)