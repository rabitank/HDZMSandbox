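; BP_PGBase is the base placement generator for the STG system, handing out a position and direction on each Pop.
; Reset stores center, direction, yaw range, count, yaw offset and radius, rejecting counts below one.
; The base Pop returns zero vectors and advances the index, which wraps at the count and fires a completion call.
; Comments indicate concrete subclasses supply their own setup, with Pop as the guaranteed shared call.
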(fn Pop
  (CallFunction|UpdateIndex)
  (return "0, 0, 0" "0, 0, 0"))

(fn Reset
  (params (CentLocal :type Vector) (CentDirect :type Rotator) (YawRange :type Float%20%28single-precision%29) (Num :type Integer) (YawOffset :type Float%20%28single-precision%29) (radius :type Float%20%28single-precision%29))
  (Variables|Default|SetCentLocal CentLocal)
  (Variables|Default|SetCentDirect CentDirect)
  (Variables|Default|SetYawRange YawRange)
  (if (>= Num 1)
    (Variables|Default|SetNum Num)
    (Variables|Default|SetDirectionYawOffset YawOffset)
    (Variables|Default|Setradius radius)
    (Variables|Default|SetCurIndex 0)
    (else
      (Development|PrintString 0 "PG's Num shouldn't negative or zero"))))

(fn Restart
  (Variables|Default|SetCurIndex 0))

(fn SetRadius
  (params (radius :type Float%20%28single-precision%29))
  (Variables|Default|Setradius radius))

(fn SetIndex
  (params (CurIndex :type Integer))
  (Variables|Default|SetCurIndex (Math|Integer|Clamp(Integer) CurIndex 0 (Variables|Default|GetNum))))

(fn UpdateIndex
  (bind _output_get (Variables|Default|SetCurIndex (+ (stale _output_get) 1)))
  (if (not (< (Variables|Default|GetCurIndex) (Variables|Default|GetNum)))
    (Variables|Default|SetCurIndex 0)
    (Default|CallPGCompleted)))