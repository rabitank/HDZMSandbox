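; BP_PG_arc is an STG placement generator that yields positions and directions spaced along an arc around a center.
; Reset derives the yaw stride from range and count, and zeroes the roll, which SetRollAngle can change to tilt the arc.
; Each Pop rotates a radius vector about the rolled up axis from minus half the range, offsets the facing yaw, then calls the parent Pop.
; ResetYawRange changes the spread and recomputes the stride.
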(fn Pop
  (bind _roll_angle (Variables|Default|GetRoll%20Angle))
  (bind _curindex (Variables|Default|GetCurIndex))
  (bind _centdirect (Variables|Default|GetCentDirect))
  (bind _yaw_stride (Variables|Default|GetYaw%20Stride))
  (bind _yawrange (Variables|Default|GetYawRange))
  (bind _returnvalue (* _curindex _yaw_stride))
  (bind _returnvalue_2 (/ _yawrange -2.0))
  (bind _returnvalue_3 (+ _roll_angle (.roll _centdirect)))
  (bind _returnvalue_4 (Math|Rotator|MakeRotator _returnvalue_3 (.pitch _centdirect) (.yaw _centdirect)))
  (bind _returnvalue_5 (+ _returnvalue _returnvalue_2))
  (bind _returnvalue_6 (Math|Vector|GetUpVector _returnvalue_4))
  (bind _output_get (LocalVariables|SetNewLocalVar_0 (+ (Math|Vector|RotateVectorAroundAxis (* (Math|Vector|GetForwardVector _returnvalue_4) (Variables|Default|Getradius)) _returnvalue_5 _returnvalue_6) (Variables|Default|GetCentLocal))))
  (bind _output_get_2 (LocalVariables|SetNewLocalVar_1 (Math|Rotator|CombineRotators (Math|Vector|RotatorfromAxisandAngle _returnvalue_6 (+ _returnvalue_5 (Variables|Default|GetDirectionYawOffset))) (Math|Rotator|MakeRotator 0.0 (.pitch _centdirect) (.yaw _centdirect)))))
  (|CallParentFunction)
  (return _output_get _output_get_2))

(fn Reset
  (params (CentLocal :type Vector :default "0, 0, 0") (CentDirect :type Rotator :default "0, 0, 0") (YawRange :type Float%20%28single-precision%29) (Num :type Integer) (YawOffset :type Float%20%28single-precision%29) (radius :type Float%20%28single-precision%29))
  (|CallParentFunction CentLocal CentDirect YawRange Num YawOffset radius)
  (Variables|Default|SetYaw%20Stride (/ (Variables|Default|GetYawRange) (Math|Conversions|ToFloat(Integer) (Variables|Default|Getnum))))
  (Variables|Default|SetRoll%20Angle 0.0))

(fn SetRollAngle
  (params (RollAngle :type Float%20%28single-precision%29))
  (Variables|Default|SetRoll%20Angle RollAngle))

(fn ResetYawRange
  (params (YawRange :type Float%20%28single-precision%29))
  (Variables|Default|SetYawRange YawRange)
  (Variables|Default|SetYaw%20Stride (/ (Variables|Default|GetYawRange) (Math|Conversions|ToFloat(Integer) (Variables|Default|Getnum)))))