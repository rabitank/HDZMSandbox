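; Placement generator for the STG system that hands out positions and directions on a UV-sphere patch of latitude/longitude grid points around a center.
; Each Pop maps the current index to yaw and pitch steps centered on the equator, converts them to a point at Radius, rotates it by AxisRot and advances the index.
; Isdiffuse selects outward-facing or shared axis direction.
; Setters refresh the cached strides and axis rotation, which combines center direction with roll.
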(fn Pop
  (bind _numpreline (Variables|Default|GetnumPreLine))
  (bind _curindex (Variables|Default|GetCurIndex))
  (bind _axisrot (Variables|Default|GetAxisRot))
  (bind _output_get (LocalVariables|Settheta (+ (* (Math|Integer|%(Integer) _curindex _numpreline) (Variables|Default|GetYaw%20Stride)) (/ (Variables|Default|GetYawRange) -2.0))))
  (bind _output_get_2 (LocalVariables|Setphi (+ (* (/ _curindex _numpreline) (Variables|Default|GetPitch%20Stride)) (/ (Variables|Default|GetPitchRange) -2.0) 9e+01)))
  (LocalVariables|SetNewLocalVar_0 (+ (Variables|Default|GetCentLocal) (Math|Vector|RotateVector (* (CallFunction|MakeUVPos _output_get_2 _output_get) (Variables|Default|Getradius)) _axisrot)))
  (if (Variables|Default|GetIsdiffuse)
    (LocalVariables|SetNewLocalVar_1 (Math|Rotator|MakeRotfromX (Math|Vector|RotateVector (* (CallFunction|MakeUVPos _output_get_2 _output_get) (Variables|Default|Getradius)) _axisrot)))
    (else
      (LocalVariables|SetNewLocalVar_1 _axisrot)))
  (CallFunction|UpdateIndex)
  (return (LocalVariables|GetNewLocalVar_0) (LocalVariables|GetNewLocalVar_1)))

(fn SetPitchRange
  (params (PitchRange :type Float%20%28single-precision%29))
  (Variables|Default|SetPitchRange PitchRange)
  (CallFunction|UpdatePitchStride))

(fn SetYawRange
  (params (YawRange :type Float%20%28single-precision%29))
  (Variables|Default|SetYawRange YawRange)
  (CallFunction|UpdateYawStride))

(fn SetLineNum
  (params (LineNum :type Integer))
  (Variables|Default|SetLineNum LineNum)
  (CallFunction|UpdatePitchStride))

(fn SetNumPreLine
  (params (NumPreLine :type Integer))
  (Variables|Default|SetNumPreLine NumPreLine)
  (CallFunction|UpdateYawStride))

(fn UpdateYawStride
  (Variables|Default|SetYaw%20Stride (/ (Variables|Default|GetYawRange) (Math|Conversions|ToFloat(Integer) (Variables|Default|GetnumPreLine)))))

(fn UpdatePitchStride
  (Variables|Default|SetPitch%20Stride (/ (Variables|Default|GetPitchRange) (Math|Conversions|ToFloat(Integer) (Variables|Default|GetLineNum)))))

(fn ResetPG
  (params (CentLocal :type Vector) (CentDirect :type Rotator) (YawRangeIn :type Float%20%28single-precision%29) (PitchRangeIn :type Float%20%28single-precision%29) (NumPreLineIn :type Integer) (LineNumIn :type Integer) (radius :type Float%20%28single-precision%29) (RollAngleIn :type Float%20%28single-precision%29) (Isdiffuse :type Boolean))
  (CallFunction|Reset CentLocal CentDirect YawRangeIn (* NumPreLineIn LineNumIn) 0.0 radius)
  (Utilities|FlowControl|Sequence
    (:then_0
      (Variables|Default|SetPitchRange PitchRangeIn)
      (Variables|Default|SetNumPreLine NumPreLineIn)
      (Variables|Default|SetLineNum LineNumIn)
      (Variables|Default|SetRoll%20Angle RollAngleIn))
    (:then_1
      (CallFunction|UpdateYawStride)
      (CallFunction|UpdatePitchStride)
      (CallFunction|UpdateAxisRot))
    (:then_2
      (Variables|Default|SetIsdiffuse Isdiffuse))))

(fn SetRollAngle
  (params (Roll%20Angle :type Float%20%28single-precision%29))
  (Variables|Default|SetRoll%20Angle Roll%20Angle)
  (CallFunction|UpdateAxisRot))

(fn UpdateAxisRot
  (bind _centdirect (Variables|Default|GetCentDirect))
  (Variables|Default|SetAxisRot (Math|Rotator|MakeRotator (Variables|Default|GetRoll%20Angle) (.pitch _centdirect) (.yaw _centdirect))))

(fn MakeUVPos
  (params (Phi :type Float%20%28single-precision%29) (Theta :type Float%20%28single-precision%29))
  (bind _returnvalue (Math|Trig|Sin(Degrees) Phi))
  (return (Math|Vector|MakeVector (* (Math|Trig|Cos(Degrees) Theta) _returnvalue) (* _returnvalue (Math|Trig|Sin(Degrees) Theta)) (Math|Trig|Cos(Degrees) Phi))))

(fn SetDirection
  (params (CentDirect :type Rotator))
  (Variables|Default|SetCentDirect CentDirect)
  (CallFunction|UpdateAxisRot))