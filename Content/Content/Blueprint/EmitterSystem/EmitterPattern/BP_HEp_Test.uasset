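; Test emitter pattern actor, owned by an HEmitter, that spins while active and animates its size between active and relaxed states.
; Tick scales sender lengths by the owner's final scale factor, then adds roll while active or eases roll back to zero.
; One ToRelax timeline, played forward or reversed, lerps scale between RelaxSize and full size, deferring the matching parent PatternRelax or PatternActive call until it finishes.
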(event EventBeginPlay)

(event Collision|EventActorBeginOverlap
  (params (OtherActor :type Actor%20Object%20Reference)))

(event EventTick
  (params (DeltaSeconds :type Float%20%28single-precision%29))
  (|CallParentFunction DeltaSeconds)
  (bind _ashemitter (Utilities|Casting|CastToHEmitter (Components|GetOwner)))
  (Class|HEmitterPattern|SetSenderLengths (* (Variables|Default|GetSenderLength) (Variables|/Script/HDZMSandbox.HEmitter|GetFinalScaleFac _ashemitter)))
  (if (Variables|Default|GetbIsActive)
    (Transformation|AddActorLocalRotation "0,0.000000,4.000000" false false)
    (else
      (Transformation|SetActorRelativeRotation (Math|Rotator|MakeRotator (Math|Interpolation|FInterpTo (.roll (Variables|/Script/Engine.SceneComponent|GetRelativeRotation (Variables|Transformation|GetRootComponent))) 0.0 (Utilities|Time|GetWorldDeltaSeconds) 1e+01) 0.0 0.0)))))

(event EventPatternActive
  (bind (_direction _scale) (Timeline|ToRelax ReverseFromEnd)
    (:Update
      (Transformation|SetActorRelativeScale3D (Math|Conversions|ToVector(Float) (Math|Float|Lerp (Variables|Default|GetRelaxSize) 1.0 _scale))))
    (:Finished
      (switch Utilities|FlowControl|Switch|SwitchonETimelineDirection _direction
        (:Forward
          (|CallParentFunction))
        (:Backward
          (|CallParentFunction))))))

(event EventPatternRelax
  (bind (_direction _scale) (Timeline|ToRelax PlayFromStart)
    (:Update
      (Transformation|SetActorRelativeScale3D (Math|Conversions|ToVector(Float) (Math|Float|Lerp (Variables|Default|GetRelaxSize) 1.0 _scale))))
    (:Finished
      (switch Utilities|FlowControl|Switch|SwitchonETimelineDirection _direction
        (:Forward
          (|CallParentFunction))
        (:Backward
          (|CallParentFunction))))))

(fn ConstructionScript)