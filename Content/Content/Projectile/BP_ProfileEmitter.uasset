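; BP_ProfileEmitter is a projectile emitter actor that fires magic projectiles at the player while switched on.
; A looping two-second timer started at BeginPlay spawns BP_MagicProjectile at the actor's transform whenever IsEmitting is set.
; Tick turns the actor toward the first player pawn each frame, so each shot launches facing the player.
; Interact toggles emission on and off through a FlipFlop.
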(event Custom|ForceEplaed
  (if (Variables|Default|GetIsEmitting)
    (Game|SpawnActorfromClass "/Game/Content/Projectile/BP_MagicProjectile.BP_MagicProjectile_C" (Transformation|GetActorTransform) "Undefined" 0 0)))

(event EventBeginPlay
  (Utilities|Time|SetTimerbyEvent (delegate Custom|ForceEplaed) 2.0 true))

(event EventTick
  (params (DeltaSeconds :type Float%20%28single-precision%29))
  (Transformation|SetActorRotation (Math|Rotator|MakeRotfromX (- (Transformation|GetActorLocation (Game|Player|GetPlayerPawn 0)) (Transformation|GetActorLocation)))))

(event EventInteract
  (params (InstigatorPawn :type Pawn%20Object%20Reference))
  (Utilities|FlowControl|FlipFlop
    (:A
      (Variables|Default|SetIsEmitting true))
    (:B
      (Variables|Default|SetIsEmitting false))))

(fn ConstructionScript)