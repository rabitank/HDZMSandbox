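; Anim notify state, named EarlyBlendOut, that stops a montage early during its window based on the owner's locomotion state.
; Each tick reads movement state, stance and movement input through Blueprint interface messages.
; A matching state or stance, or any movement input, stops the montage with a configurable blend-out time.
; CheckMovementInput gates both movement-state and input tests, while CheckMovementState gates the stance test.
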(fn ReceivedNotifyTick
  (params (MeshComp :type Skeletal%20Mesh%20Component%20Object%20Reference) (Animation :type Anim%20Sequence%20Base%20Object%20Reference) (FrameDeltaTime :type Float%20%28single-precision%29))
  (LocalVariables|SetAnimInstance (Components|SkeletalMesh|GetAnimInstance MeshComp))
  (LocalVariables|SetOwnerActor (Components|GetOwner MeshComp))
  (Utilities|FlowControl|Sequence
    (:then_0
      (if (Variables|Default|GetCheckMovementInput)
        (bind _movementstate (Class|HLSCharacterBPI|BPIGetCurrentState(Message) (LocalVariables|GetOwnerActor)))
        (if (Utilities|Enum|Equal(Enum) (Variables|Default|GetMovementStateEquals) _movementstate)
          (Animation|Montage|MontageStop (LocalVariables|GetAnimInstance) (Variables|Default|GetBlendOuTime) (Variables|Default|GetThisMontage)))))
    (:then_1
      (if (Variables|Default|GetCheckMovementState)
        (bind _actual_stance (Class|HLSCharacterBPI|BPIGetCurrentState(Message) (LocalVariables|GetOwnerActor)))
        (if (Utilities|Enum|Equal(Enum) (Variables|Default|GetStanceEquals) _actual_stance)
          (Animation|Montage|MontageStop (LocalVariables|GetAnimInstance) (Variables|Default|GetBlendOuTime) (Variables|Default|GetThisMontage)))))
    (:then_2
      (if (Variables|Default|GetCheckMovementInput)
        (bind _hasmovementinput (Class|HLSCharacterBPI|BPIGetEssentialValues(Message) (LocalVariables|GetOwnerActor)))
        (if _hasmovementinput
          (Animation|Montage|MontageStop (LocalVariables|GetAnimInstance) (Variables|Default|GetBlendOuTime) (Variables|Default|GetThisMontage)))))))

(fn GetNotifyName
  (return "EarlyBlendOut"))