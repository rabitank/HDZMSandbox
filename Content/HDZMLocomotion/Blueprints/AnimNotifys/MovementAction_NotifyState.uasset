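; Anim notify state that sets the owning actor's Movement Action enum for the length of an animation window.
; On begin it sends the configured action to the mesh owner through a Blueprint interface message.
; On end it resets to a default enum value only if the owner's current action still matches, so a later state change is not overwritten.
; The notify's editor name shows the configured action.
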(fn ReceivedNotifyBegin
  (params (MeshComp :type Skeletal%20Mesh%20Component%20Object%20Reference) (Animation :type Anim%20Sequence%20Base%20Object%20Reference) (TotalDuration :type Float%20%28single-precision%29))
  ;[1 1 1] 获取Comp的owning Actor,并尝试调用接口以修改Action枚举,实现状态更新
  (Class|HLSCharacterBPI|BPISetMovementAction(Message) (Components|GetOwner MeshComp) (Variables|Default|GetMovement%20Action))
  (return false))

(fn ReceivedNotifyEnd
  (params (MeshComp :type Skeletal%20Mesh%20Component%20Object%20Reference) (Animation :type Anim%20Sequence%20Base%20Object%20Reference))
  (bind _returnvalue (Components|GetOwner MeshComp))
  (bind _movement_action (Class|HLSCharacterBPI|BPIGetCurrentState(Message) _returnvalue))
  (if (Utilities|Enum|Equal(Enum) _movement_action (Variables|Default|GetMovement%20Action))
    (Class|HLSCharacterBPI|BPISetMovementAction(Message) _returnvalue "NewEnumerator4")
    (return false)
    (else
      (return false))))

(fn GetNotifyName
  (return (Utilities|String|Append "Movement Action" (Utilities|String|EnumtoString (Variables|Default|GetMovement%20Action)))))