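; Footstep anim notify that plays a footstep sound attached to a point on the animated mesh.
; Volume is scaled by one minus the anim instance's Mask_FootstepSound curve, unless OverrideMaskCurve applies the plain multiplier.
; The spawned audio component receives the footstep type as an integer FootstepType parameter, letting the sound asset vary by type.
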(fn ReceivedNotify
  (params (MeshComp :type Skeletal%20Mesh%20Component%20Object%20Reference) (Animation :type Anim%20Sequence%20Base%20Object%20Reference))
  (bind _returnvalue (Components|SkeletalMesh|GetAnimInstance MeshComp))
  (bind _sound (Variables|Default|GetSound))
  (Utilities|IsValid MeshComp
    (:Is%20Valid
      (Utilities|IsValid _returnvalue
        (:Is%20Valid
          ;[1 1 1] 确认有效后,将声音附到模型骨骼上,并配置后参数
          (Utilities|IsValid _sound
            (:Is%20Valid
              (bind _returnvalue_2 (Audio|SpawnSoundAttached _sound MeshComp (Variables|Default|GetAttachPointName) "0, 0, 0" "0, 0, 0" "KeepRelativeOffset" false (select (Variables|Default|GetOverrideMaskCurve) (Variables|Default|GetVolumeMultiplier) (* (- 1.0 (Animation|Curves|GetCurveValue _returnvalue "Mask_FootstepSound")) (Variables|Default|GetVolumeMultiplier))) (Variables|Default|GetPitchMultiplier) 0.0 0 0))
              ;[1 1 1] 这应该是SoundBase里的参数
              (Utilities|IsValid _returnvalue_2
                (:Is%20Valid
                  (Effects|Components|ParticleSystem|SetIntParameter _returnvalue_2 "FootstepType" (Math|Conversions|ToInteger(Byte) (Variables|Default|GetFootSteptype)))
                  (return false))))))))))