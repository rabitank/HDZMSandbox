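; Locomotion character child Blueprint that adds held objects and overlay-specific animation choices to its parent.
; Overlay state picks mantle, roll and get-up assets, plus the pistol, bow, torch or box mesh attached to virtual-bone hand sockets.
; High or falling mantles and ragdoll clear the held object, restored when they end.
; It also supplies socket-based camera targets through interface overrides and can drive bow draw from an animation curve.
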(event EventBeginPlay)

(event Collision|EventActorBeginOverlap
  (params (OtherActor :type Actor%20Object%20Reference)))

(event EventTick
  (params (DeltaSeconds :type Float%20%28single-precision%29)))

(fn ConstructionScript
  (|CallParentFunction))

(fn BPIGet3PTraceParameters
  ;[1 1 1] 获取第三人称下的左右肩追踪参数
  (if (Variables|Default|GetRight%20Shoulder)
    (return (Transformation|GetSocketLocation (Variables|Character|GetMesh) "TP_CameraTrace_R") 1e+01 "TraceTypeQuery1")
    (else
      (return (Transformation|GetSocketLocation (Variables|Character|GetMesh) "TP_CameraTrace_R") 1e+01 "TraceTypeQuery1"))))

(fn BPIGet3PPivotTarget
  (bind _mesh (Variables|Character|GetMesh))
  ;[1 1 1] 获取第三人称锚点位姿
  (return (Math|Transform|MakeTransform (Math|Vector|GetVectorArrayAverage (Utilities|Array|MakeArray (Transformation|GetSocketLocation _mesh "head") (Transformation|GetSocketLocation _mesh "root"))) (Transformation|GetActorRotation))))

(fn BPIGetFPCameraTarget
  ;[1 1 1] 获取第一人称下的摄像机位置
  (return (Transformation|GetSocketLocation (Variables|Character|GetMesh) "FP_Camera")))

(fn BPIGetCameraParameters
  (bind (_rightshoulder _tp_fov) (|CallParentFunction))
  (return _rightshoulder _tp_fov))

(fn MantleStart
  (params (Mantle%20Height :type Float%20%28single-precision%29) (Mantle%20Ledge%20WS%28world%20Space%29 :type HLS%20Component%20and%20Transform%20Structure) (Mantle%20Type :type HLS_MantleType%20Enum :default "NewEnumerator0"))
  (|CallParentFunction Mantle%20Height Mantle%20Ledge%20WS%28world%20Space%29 Mantle%20Type)
  (switch Utilities|FlowControl|Switch|SwitchonHLS_MantleType Mantle%20Type
    (:NewEnumerator0
      _)
    (:NewEnumerator2
      _))
  (CallFunction|ClearHeldObject))

(fn MantleEnd
  (|CallParentFunction)
  (CallFunction|UpdateHeldObject))

(fn GetMantleAsset
  (params (Mantle%20Type :type HLS_MantleType%20Enum :default "NewEnumerator0"))
  (switch Utilities|FlowControl|Switch|SwitchonHLS_MantleType Mantle%20Type
    (:NewEnumerator0
      _)
    (:NewEnumerator1
      (switch Utilities|FlowControl|Switch|SwitchonHLS_OverlayState (Variables|Default|GetOverlay%20State)
        (:NewEnumerator0
          _)
        (:NewEnumerator1
          _)
        (:NewEnumerator2
          _)
        (:NewEnumerator3
          (return (Variables|Mantle|GetMantle%201m%20LH)))
        (:NewEnumerator4
          (return (Variables|Mantle|GetMantle%201m%202H)))
        (:NewEnumerator6
          (return (Variables|Mantle|GetMantle%201m%20RH)))
        (:NewEnumerator7
          (return (Variables|Mantle|GetMantle%201m%20RH)))
        (:NewEnumerator8
          (return (Variables|Mantle|GetMantle%201m%20LH)))
        (:NewEnumerator9
          (return (Variables|Mantle|GetMantle%201m%20LH)))
        (:NewEnumerator11
          (return (Variables|Mantle|GetMantle%201m%20Box))))
      (return (Variables|Mantle|GetMantle%201m%20Default)))
    (:NewEnumerator2
      _))
  (return (Variables|Mantle|GetMantle%202m%20Default)))

(fn GetRollAnimation
  (switch Utilities|FlowControl|Switch|SwitchonHLS_OverlayState (Variables|Default|GetOverlay%20State)
    (:NewEnumerator0
      _)
    (:NewEnumerator1
      _)
    (:NewEnumerator2
      _)
    (:NewEnumerator3
      (return (Variables|LandRoll|GetLandRoll%20LH)))
    (:NewEnumerator4
      (return (Variables|LandRoll|GetLandRoll%202H)))
    (:NewEnumerator6
      (return (Variables|LandRoll|GetLandRoll%20RH)))
    (:NewEnumerator7
      (return (Variables|LandRoll|GetLandRoll%20RH)))
    (:NewEnumerator8
      (return (Variables|LandRoll|GetLandRoll%20LH)))
    (:NewEnumerator9
      (return (Variables|LandRoll|GetLandRoll%20LH)))
    (:NewEnumerator11
      (return (Variables|LandRoll|GetLandRoll%202H))))
  (return (Variables|LandRoll|GetLandRoll%20Default)))

(fn UpdateHeldObject
  (switch Utilities|FlowControl|Switch|SwitchonHLS_OverlayState (Variables|Default|GetOverlay%20State)
    (:NewEnumerator0
      (CallFunction|ClearHeldObject :!label _label))
    (:NewEnumerator1
      (goto _label))
    (:NewEnumerator2
      (goto _label))
    (:NewEnumerator3
      (goto _label))
    (:NewEnumerator4
      (goto _label))
    (:NewEnumerator6
      (CallFunction|AttachtoHand 0 "/Game/HDZMLocomotion/Props/Meshes/M9.M9" 0 false "0, 0, 0"))
    (:NewEnumerator7
      (CallFunction|AttachtoHand 0 "/Game/HDZMLocomotion/Props/Meshes/M9.M9" 0 false "0, 0, 0"))
    (:NewEnumerator8
      (CallFunction|AttachtoHand 0 "/Game/HDZMLocomotion/Props/Meshes/Bow.Bow" "/Game/HDZMLocomotion/Props/Meshes/Bow_AnimBP.Bow_AnimBP_C" true "0, 0, 0"))
    (:NewEnumerator9
      (CallFunction|AttachtoHand "/Game/HDZMLocomotion/Props/Meshes/Torch.Torch" 0 0 true "0, 0, 0"))
    (:NewEnumerator11
      (CallFunction|AttachtoHand "/Game/HDZMLocomotion/Props/Meshes/Box.Box" 0 0 false "0, 0, 0"))))

(fn ClearHeldObject
  (bind _skeletalmesh (Variables|Default|GetSkeletalMesh))
  (Class|SkinnedMeshComponent|SetSkeletalMesh _skeletalmesh 0 false)
  (Class|SkeletalMeshComponent|SetAnimClass _skeletalmesh)
  (Components|StaticMesh|SetStaticMesh (Variables|Default|GetStaticMesh) 0))

(fn AttachtoHand
  (params (NewStaticMesh :type Static%20Mesh%20Object%20Reference) (NewSkeletalMesh :type Skeletal%20Mesh%20Object%20Reference) (NewAnimClass :type Object%20Class%20Reference) (LeftHand :type Boolean) (Offset :type Vector))
  (Utilities|FlowControl|Sequence
    (:then_0
      (CallFunction|ClearHeldObject))
    (:then_1
      (bind _newstaticmesh (LocalVariables|GetNewStaticMesh)
        (:then
          (Components|StaticMesh|SetStaticMesh (Variables|Default|GetStaticMesh) _newstaticmesh))
        (:else)))
    (:then_2
      (bind _newskeletalmesh (LocalVariables|GetNewSkeletalMesh)
        (:then
          (Class|SkinnedMeshComponent|SetSkeletalMesh (Variables|Default|GetSkeletalMesh) _newskeletalmesh true)
          ;[1 1 1] 动态设置手持物的动画实例
          (bind _newanimclass (LocalVariables|GetNewAnimClass)
            (:then
              (Class|SkeletalMeshComponent|SetAnimClass (Variables|Default|GetSkeletalMesh) _newanimclass))
            (:else)))
        (:else)))
    (:then_3
      ;[1 1 1] 绑定HO并设置偏移
      (Transformation|AttachComponentToComponent (Variables|Default|GetHeldObjectRoot) (Variables|Character|GetMesh) (select LeftHand "VB LHS_ik_hand_gun" "VB RHS_ik_hand_gun") "SnapToTarget" "SnapToTarget" "SnapToTarget" true) ; 进入相对坐标系,标准的SceneComp的Attach
      (Transformation|SetRelativeLocation (Variables|Default|GetHeldObjectRoot) Offset false false))))

(fn UpdateHeldObjectAnimations
  (switch Utilities|FlowControl|Switch|SwitchonHLS_OverlayState (Variables|Default|GetOverlay%20State)
    (:NewEnumerator8
      (bind _asbow_anim_bp (Utilities|Casting|CastToBow_AnimBP (Components|SkeletalMesh|GetAnimInstance (Variables|Default|GetSkeletalMesh))))
      (Variables|/Game/HDZMLocomotion/Props/Meshes/Bow_AnimBP.Bow_AnimBP_C|SetDraw _asbow_anim_bp (CallFunction|GetAnimCurvesValue "Enable_SpineRotation")))))

(fn OnOverlayStateChanged
  (params (Overlay%20State :type HLS_OverlayState%20Enum :default "NewEnumerator0"))
  (|CallParentFunction Overlay%20State)
  (CallFunction|UpdateHeldObject))

(fn GetGetupMontage
  (params (Face%20up :type Boolean))
  (if Face%20up ; face up 是指需要抬起脸的意思?
    (switch Utilities|FlowControl|Switch|SwitchonHLS_OverlayState (Variables|Default|GetOverlay%20State)
      (:NewEnumerator0
        _)
      (:NewEnumerator1
        _)
      (:NewEnumerator2
        _)
      (:NewEnumerator3
        (return (Variables|Default|GetGetup%20B%20LH)))
      (:NewEnumerator4
        (return (Variables|Default|GetGetup%20B%202H)))
      (:NewEnumerator6
        (return (Variables|Default|GetGetup%20B%20RH)))
      (:NewEnumerator7
        (return (Variables|Default|GetGetup%20B%20RH)))
      (:NewEnumerator8
        (return (Variables|Default|GetGetup%20B%20LH)))
      (:NewEnumerator9
        (return (Variables|Default|GetGetup%20B%20LH)))
      (:NewEnumerator11
        (return (Variables|Default|GetGetup%20B%202H))))
    (return (Variables|Default|GetGetup%20B%20Default))
    (else
      (switch Utilities|FlowControl|Switch|SwitchonHLS_OverlayState (Variables|Default|GetOverlay%20State)
        (:NewEnumerator0
          _)
        (:NewEnumerator1
          _)
        (:NewEnumerator2
          _)
        (:NewEnumerator3
          (return (Variables|Default|GetGetup%20F%20LH)))
        (:NewEnumerator4
          (return (Variables|Default|GetGetup%20F%202H)))
        (:NewEnumerator6
          (return (Variables|Default|GetGetup%20F%20RH)))
        (:NewEnumerator7
          (return (Variables|Default|GetGetup%20F%20RH)))
        (:NewEnumerator8
          (return (Variables|Default|GetGetup%20F%20LH)))
        (:NewEnumerator9
          (return (Variables|Default|GetGetup%20F%20LH)))
        (:NewEnumerator11
          (return (Variables|Default|GetGetup%20F%202H))))
      (return (Variables|Default|GetGetup%20F%20Default)))))

(fn RagDollStart
  (CallFunction|ClearHeldObject)
  (|CallParentFunction))

(fn RagDollEnd
  (|CallParentFunction)
  (CallFunction|UpdateHeldObject))