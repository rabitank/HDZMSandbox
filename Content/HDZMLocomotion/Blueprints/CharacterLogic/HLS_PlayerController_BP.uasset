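; Player controller for the HLS locomotion system, handling HUD creation, debug toggles and the overlay-state menu.
; BeginPlay adds the HUD and caches debug characters, while possession notifies the custom camera manager.
; Keys flip HUD, trace, shape and slow-motion flags; holding the menu input slows time and shows a cyclable switcher.
; Release applies and closes it only outside slow motion; the debug-info interface returns all false rather than those flags.
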(event EventBeginPlay
  (bind _returnvalue (UserInterface|CreateWidget "/Game/HDZMLocomotion/Blueprints/UI/HLS_HUD.HLS_HUD_C" self))
  (bind _output_get (Variables|Default|SetALS_HUD _returnvalue))
  (UserInterface|Viewport|AddtoViewport _output_get 0)
  (bind _outactors (Actor|GetAllActorsOfClass "/Game/HDZMLocomotion/Blueprints/CharacterLogic/HLS_Base_Character_BP.HLS_Base_Character_BP_C"))
  (Variables|Debug|SetAvaliable%20Debug%20Characters _outactors)
  (Variables|Debug|SetDebug%20Focus%20Character (Game|GetPlayerCharacter 0)))

(event EventTick
  (params (DeltaSeconds :type Float%20%28single-precision%29)))

(event EventPossess
  (params (PossessedPawn :type Pawn%20Object%20Reference))
  (bind _ashls_player_camera_manager_bp (Utilities|Casting|CastToHLS_PlayerCameraManager_BP (Variables|Default|GetPlayerCameraManager)))
  (Default|OnPoccesed _ashls_player_camera_manager_bp PossessedPawn))

(event Input|ActionEvents|InputActionOpenOverlayerMenu
  (params (Key :type Key%20Structure))
  (:Pressed
    (Variables|Default|SetOpenoverlayerMenu true)
    (if (Variables|Debug|GetSlomo)
      _
      (else
        (Utilities|Time|SetGlobalTimeDilation 0.35)))
    (bind _returnvalue (UserInterface|CreateWidget "/Game/HDZMLocomotion/Blueprints/UI/OverlayStateSwitcher.OverlayStateSwitcher_C" self))
    (bind _output_get (Variables|Default|SetOverlay%20State%20Widget _returnvalue))
    (UserInterface|Viewport|AddtoViewport _output_get 0)
    (Audio|PlaySound2D "/Game/HDZMLocomotion/Audio/UI/Click.Click" 1.0 1.0 0.0 0 0))
  (:Released
    (Variables|Default|SetOpenoverlayerMenu false)
    (if (not (Variables|Debug|GetSlomo))
      (Utilities|Time|SetGlobalTimeDilation 1.0)
      (Default|SelectOverlayState (Variables|Default|GetOverlay%20State%20Widget))
      (Widget|RemovefromParent (Variables|Default|GetOverlay%20State%20Widget))
      (Audio|PlaySound2D "/Game/HDZMLocomotion/Audio/UI/Click.Click" 1.0 1.0 0.0 0 0))))

(event Input|ActionEvents|InputActionSelectedCycleDown
  (params (Key :type Key%20Structure))
  (:Pressed
    (if (Variables|Default|GetOpenoverlayerMenu)
      (bind _overlay_state_widget (Variables|Default|GetOverlay%20State%20Widget)
        (:then
          (Default|CycleState _overlay_state_widget false)
          (Audio|PlaySound2D "/Game/HDZMLocomotion/Audio/UI/Click.Click" 1.0 1.0 0.0 0 0))
        (:else)))))

(event Input|ActionEvents|InputActionSelectedCycleUp
  (params (Key :type Key%20Structure))
  (:Pressed
    (if (Variables|Default|GetOpenoverlayerMenu)
      (bind _overlay_state_widget (Variables|Default|GetOverlay%20State%20Widget)
        (:then
          (Default|CycleState _overlay_state_widget true)
          (Audio|PlaySound2D "/Game/HDZMLocomotion/Audio/UI/Click.Click" 1.0 1.0 0.0 0 0))
        (:else)))))

(event Input|KeyboardEvents|Tab
  (params (Key :type Key%20Structure))
  (:Pressed
    (Variables|Debug|SetShow%20HUD (not (Variables|Debug|GetShow%20HUD)))))

(event Input|KeyboardEvents|V
  (params (Key :type Key%20Structure))
  (:Pressed
    (Variables|Debug|SetShow%20Traces (not (Variables|Debug|GetShow%20Traces)))))

(event Input|KeyboardEvents|Y
  (params (Key :type Key%20Structure))
  (:Pressed
    (Variables|Debug|SetShow%20Debug%20Shapes (not (Variables|Debug|GetShow%20Debug%20Shapes)))))

(event Input|KeyboardEvents|Z
  (params (Key :type Key%20Structure))
  (:Pressed
    (bind _output_get (Variables|Debug|SetSlomo (not (Variables|Debug|GetSlomo))))
    (if _output_get
      ;[1 1 1] 时间膨胀-> 子弹时间效果
      (Utilities|Time|SetGlobalTimeDilation 0.1)
      (else
        (Utilities|Time|SetGlobalTimeDilation 1.0)))))

(fn ConstructionScript)

(fn BPIGetDebugInfo
  (return 0 false false false false false false false))