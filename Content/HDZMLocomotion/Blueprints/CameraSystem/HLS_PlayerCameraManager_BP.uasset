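; Player camera manager that drives a custom third-person camera for pawns tagged HSL_Character and defers to the parent update otherwise.
; Pivot, FOV and trace settings come from the pawn through interface calls, while offsets and lag speeds are read as CameraBehavior AnimBP curves.
; It lags rotation and per-axis pivot in camera-yaw space, blends toward a debug view via Override_Debug, then sphere-traces to prevent clipping.
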(event Custom|OnPoccesed
  (params (ControllerPawn :type Pawn%20Object%20Reference))
  (Variables|Default|SetControllerPawn ControllerPawn)
  (bind _ashls_player_camer_behavior_bp (Utilities|Casting|CastToHLS_PlayerCamerBehavior_BP (Components|SkeletalMesh|GetAnimInstance (Variables|Default|GetCameraBehavior))))
  (Variables|/Game/HDZMLocomotion/Blueprints/CameraSystem/HLS_PlayerCamerBehavior_BP.HLS_PlayerCamerBehavior_BP_C|SetPlayerController _ashls_player_camer_behavior_bp (Game|Player|GetOwningPlayerController))
  (Variables|/Game/HDZMLocomotion/Blueprints/CameraSystem/HLS_PlayerCamerBehavior_BP.HLS_PlayerCamerBehavior_BP_C|SetControlledPawn _ashls_player_camer_behavior_bp ControllerPawn))

(event EventBeginPlay)

(event Collision|EventActorBeginOverlap
  (params (OtherActor :type Actor%20Object%20Reference)))

(event EventTick
  (params (DeltaSeconds :type Float%20%28single-precision%29))
  (Development|PrintString (Utilities|String|Append (Utilities|String|Append "Override_Debug: " (Utilities|String|ToString(Float) (CallFunction|GetCameraBehvaiorParam "Override_Debug"))) " " (Utilities|String|Append "CameraOffset_Y: " (Utilities|String|ToString(Float) (CallFunction|GetCameraBehvaiorParam "CameraOffset_Y")))) true true "(R=0.000000,G=0.660000,B=1.000000,A=1.000000)" 0.0))

(fn ConstructionScript)

(fn BlueprintUpdateCamera
  (params (CameraTarget :type Actor%20Object%20Reference))
  (if (Actor|ActorHasTag (Variables|Default|GetControllerPawn) "HSL_Character")
    (bind (_return_value_location _return_value_rotation _returnvalue) (CallFunction|CustomCameraBehavior))
    (return _return_value_location _return_value_rotation _returnvalue true)
    (else
      (bind (_newcameralocation _newcamerarotation _newcamerafov _returnvalue_2) (|CallParentFunction CameraTarget))
      (return _newcameralocation _newcamerarotation _newcamerafov _returnvalue_2))))

(fn CustomCameraBehavior
  (bind _controllerpawn (Variables|Default|GetControllerPawn))
  (Utilities|FlowControl|Sequence
    (:then_0
      ;[1 1 1] 获得HSLCharacter中的相机相关数据
      (bind _return_value (Class|HLSCameraBPI|BPIGet3PPivotTarget(Message) _controllerpawn))
      (LocalVariables|SetPivotTransform _return_value)
      (bind _tp_fov (Class|HLSCameraBPI|BPIGetCameraParameters(Message) _controllerpawn))
      (LocalVariables|SetTPFOV _tp_fov)
      (bind _return_value_2 (Class|HLSCameraBPI|BPIGetFPCameraTarget(Message) _controllerpawn))
      (LocalVariables|SetFP%20Target _return_value_2))
    (:then_1
      (Variables|Default|SetTarget%20Camera%20Rotator (Math|Rotator|Lerp(Rotator) (Math|Interpolation|RInterpTo (Camera|GetCameraRotation) (Pawn|GetControlRotation (Game|Player|GetOwningPlayerController) :!class /Script/Engine.Controller) (Utilities|Time|GetWorldDeltaSeconds) (CallFunction|GetCameraBehvaiorParam "RotationLagSpeed")) (Variables|Default|GetDebug%20Camera%20Rotator) (CallFunction|GetCameraBehvaiorParam "Override_Debug"))))
    (:then_2
      ;[1 1 1] 相机平滑锚点对实际锚点的跟随:通过对character传递的mesh的锚点进行带参插值来更新平滑锚点的姿态
      (Variables|Default|SetSmooth%20Target%20Pivot (Math|Transform|MakeTransform (CallFunction|CaculateAxisLndependentLag (.location (Variables|Default|GetSmooth%20Target%20Pivot)) (.location (LocalVariables|GetPivotTransform)) (Variables|Default|GetTarget%20Camera%20Rotator) (Math|Vector|MakeVector (CallFunction|GetCameraBehvaiorParam "PivotLagSpeed_X") (CallFunction|GetCameraBehvaiorParam "PivotLagSpeed_Y") (CallFunction|GetCameraBehvaiorParam "PivotLagSpeed_Z"))) (.rotation (LocalVariables|GetPivotTransform)) (.scale (LocalVariables|GetPivotTransform)))))
    (:then_3
      ;[1 1 1] 在平滑锚点的基础上使用动画曲线进行偏移得到最后的锚点位置
      (Variables|Default|SetPivotLocation (+ (.location (Variables|Default|GetSmooth%20Target%20Pivot)) (* (Math|Vector|GetForwardVector (.rotation (Variables|Default|GetSmooth%20Target%20Pivot))) (CallFunction|GetCameraBehvaiorParam "PivotOffset_X")) (* (Math|Vector|GetUpVector (.rotation (Variables|Default|GetSmooth%20Target%20Pivot))) (CallFunction|GetCameraBehvaiorParam "PivotOffset_Z")) (* (Math|Vector|GetRightVector (.rotation (Variables|Default|GetSmooth%20Target%20Pivot))) (CallFunction|GetCameraBehvaiorParam "PivotOffset_Y")))))
    (:then_4
      (Variables|Default|SetTargetCameraLocation (Math|Vector|Lerp(Vector) (+ (Variables|Default|GetPivotLocation) (* (Math|Vector|GetForwardVector (Variables|Default|GetTarget%20Camera%20Rotator)) (CallFunction|GetCameraBehvaiorParam "CameraOffset_X")) (* (Math|Vector|GetRightVector (Variables|Default|GetTarget%20Camera%20Rotator)) (CallFunction|GetCameraBehvaiorParam "CameraOffset_Y")) (* (Math|Vector|GetUpVector (Variables|Default|GetTarget%20Camera%20Rotator)) (CallFunction|GetCameraBehvaiorParam "CameraOffset_Z"))) (+ (.location (LocalVariables|GetPivotTransform)) (Variables|Default|GetDebugCameraOffset)) (CallFunction|GetCameraBehvaiorParam "Override_Debug"))))
    (:then_5
      ;[1 1 1] 球形射线检测防止摄像机穿透
      (bind (_trace_drigin _trace_radius _trace_channel) (Class|HLSCameraBPI|BPIGet3PTraceParameters(Message) (Variables|Default|GetControllerPawn)))
      (bind _outhit (Collision|SphereTraceByChannel _trace_drigin (Variables|Default|GetTargetCameraLocation) _trace_radius _trace_channel false 0 (CallFunction|GetDebugTraceType "ForOneFrame")))
      (if (and (.bBlockingHit (Collision|BreakHitResult _outhit)) (not (.bInitialOverlap (Collision|BreakHitResult _outhit))))
        (Variables|Default|SetTargetCameraLocation (+ (- (.Location (Collision|BreakHitResult _outhit)) (.TraceEnd (Collision|BreakHitResult _outhit))) (Variables|Default|GetTargetCameraLocation)))))
    (:then_6
      ;[1 1 1] Debug Draw Shapes
      (bind _showdebugshapes (Class|HLSControllerBPI|BPIGetDebugInfo(Message) (Game|Player|GetOwningPlayerController)))
      (if _showdebugshapes
        (Rendering|Debug|DrawDebugSphere (.location (LocalVariables|GetPivotTransform)) 1e+01 12 "(R=0.054045,G=1.000000,B=0.000000,A=1.000000)" 0.0)
        (Rendering|Debug|DrawDebugSphere (.location (Variables|Default|GetSmooth%20Target%20Pivot)) 15.0 12 "(R=0.000000,G=0.864498,B=1.000000,A=1.000000)" 0.0)
        (Rendering|Debug|DrawDebugString (.location (Variables|Default|GetSmooth%20Target%20Pivot)) "Smooth Pivot Location" 0 "(R=1.000000,G=1.000000,B=1.000000,A=1.000000)")
        (Rendering|Debug|DrawDebugSphere (Variables|Default|GetPivotLocation) 18.0 12 "(R=0.383312,G=0.000000,B=1.000000,A=1.000000)" 0.0)
        (Rendering|Debug|DrawDebugString (Variables|Default|GetPivotLocation) "Pivot Location" 0 "(R=1.000000,G=1.000000,B=1.000000,A=1.000000)")
        (Rendering|Debug|DrawDebugLine (Variables|Default|GetPivotLocation) (Variables|Default|GetTargetCameraLocation) "(R=1.000000,G=0.000000,B=0.463065,A=1.000000)" 0.0 0.0)
        (Rendering|Debug|DrawDebugString (Variables|Default|GetTargetCameraLocation) "target Camera " 0 "(R=1.000000,G=1.000000,B=1.000000,A=1.000000)")))
    (:then_7
      (return (.location (Math|Transform|Lerp(Transform) (Math|Transform|MakeTransform (Variables|Default|GetTargetCameraLocation) (Variables|Default|GetTarget%20Camera%20Rotator)) (Math|Transform|MakeTransform (Variables|Default|GetTargetCameraLocation) (Variables|Default|GetDebug%20Camera%20Rotator)) (CallFunction|GetCameraBehvaiorParam "Override_Debug"))) (.rotation (Math|Transform|Lerp(Transform) (Math|Transform|MakeTransform (Variables|Default|GetTargetCameraLocation) (Variables|Default|GetTarget%20Camera%20Rotator)) (Math|Transform|MakeTransform (Variables|Default|GetTargetCameraLocation) (Variables|Default|GetDebug%20Camera%20Rotator)) (CallFunction|GetCameraBehvaiorParam "Override_Debug"))) (LocalVariables|GetTPFOV)))))

(fn GetCameraBehvaiorParam
  (params (CurveName :type Name))
  (bind _camerabehavior (Variables|Default|GetCameraBehavior))
  (bind _returnvalue (Components|SkeletalMesh|GetAnimInstance _camerabehavior))
  ;[1 1 1] 获取动画蓝图里修改过的骨骼动画曲线值
  (if (Utilities|IsValid _returnvalue)
    (return (Animation|Curves|GetCurveValue _returnvalue CurveName))
    (else
      (return 0.0))))

(fn CaculateAxisLndependentLag
  (params (CurrentLocation :type Vector) (TargetLocation :type Vector) (CameraRotation :type Rotator) (LagSpeed :type Vector))
  (bind _returnvalue (Utilities|Time|GetWorldDeltaSeconds))
  (bind _output_get (LocalVariables|SetCamera%20Rotation%20Yaw (Math|Rotator|MakeRotator 0.0 0.0 (.yaw CameraRotation))))
  (return (Math|Vector|RotateVector (Math|Vector|MakeVector (Math|Interpolation|FInterpTo (.x (Math|Vector|UnrotateVector CurrentLocation (LocalVariables|GetCamera%20Rotation%20Yaw))) (.x (Math|Vector|UnrotateVector TargetLocation (LocalVariables|GetCamera%20Rotation%20Yaw))) _returnvalue (.x LagSpeed)) (Math|Interpolation|FInterpTo (.y (Math|Vector|UnrotateVector CurrentLocation (LocalVariables|GetCamera%20Rotation%20Yaw))) (.y (Math|Vector|UnrotateVector TargetLocation (LocalVariables|GetCamera%20Rotation%20Yaw))) _returnvalue (.y LagSpeed)) (Math|Interpolation|FInterpTo (.z (Math|Vector|UnrotateVector CurrentLocation (LocalVariables|GetCamera%20Rotation%20Yaw))) (.z (Math|Vector|UnrotateVector TargetLocation (LocalVariables|GetCamera%20Rotation%20Yaw))) _returnvalue (.z LagSpeed))) _output_get)))

(fn GetDebugTraceType
  (params (Debug%20Show%20Trace%20Type :type EDrawDebugTrace%20Enum :default "None"))
  ;[1 1 1] 显示追踪轨迹?
  (bind _showtraces (Class|HLSControllerBPI|BPIGetDebugInfo(Message) (Game|GetPlayerController 0)))
  (if _showtraces
    (return Debug%20Show%20Trace%20Type)
    (else
      (return "None"))))