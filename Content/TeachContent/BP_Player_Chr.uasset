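; Player character Blueprint that adds parry input, an on-screen health widget and a save hotkey.
; The Parry input starts the "Parry" action by name on the action component.
; BeginPlay creates a minion health widget attached to the character and adds it to the viewport.
; The L key calls WriteSaveGame on SGameModeBase; debug prints accompany parry and save, and the health-changed event is empty.
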(event OnHealthChanged(ComSAttribute)
  (params (owningComp :type S%20Attribute%20Component%20Object%20Reference) (instigatorActor :type Actor%20Object%20Reference) (newAttribute :type Float%20%28single-precision%29) (delta :type Float%20%28single-precision%29)))

(event Collision|EventActorBeginOverlap
  (params (OtherActor :type Actor%20Object%20Reference)))

(event EventTick
  (params (DeltaSeconds :type Float%20%28single-precision%29)))

(event EventBeginPlay
  (bind _returnvalue (UserInterface|CreateWidget "/Game/TeachContent/UI/UI_Minionhealth.UI_Minionhealth_C" 0 self))
  (UserInterface|Viewport|AddtoViewport _returnvalue 0))

(event Input|ActionEvents|InputActionParry
  (params (Key :type Key%20Structure :default "None"))
  (:Pressed
    (Class|SActionComponent|StartActionbyName (Variables|Default|GetComActions) self "Parry")
    (Development|PrintString "Parry:Part On Character")))

(event Input|KeyboardEvents|L
  (params (Key :type Key%20Structure :default "None"))
  (:Pressed
    (bind _assgame_mode_base (Utilities|Casting|CastToSGameModeBase (Game|GetGameMode)))
    (Class|SGameModeBase|WriteSaveGame _assgame_mode_base)
    (Development|PrintString "Save Game")))

(fn ConstructionScript)