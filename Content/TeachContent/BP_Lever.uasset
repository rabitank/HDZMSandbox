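; Interactable lever that triggers a linked actor and toggles a key card gameplay tag on the pawn that uses it.
; On Interact, it forwards the interaction to SelectedActor, then a FlipFlop swings the Handle between two pitch angles.
; The same toggle alternately adds and removes KeyCardTag in the instigator's SActionComponent active tags, with state kept per lever rather than per pawn.
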(event EventBeginPlay)

(event Collision|EventActorBeginOverlap
  (params (OtherActor :type Actor%20Object%20Reference)))

(event EventTick
  (params (DeltaSeconds :type Float%20%28single-precision%29)))

(event EventInteract
  (params (InstigatorPawn :type Pawn%20Object%20Reference))
  (bind _returnvalue (Actor|GetComponentbyClass InstigatorPawn "/Script/HDZMSandbox.SActionComponent"))
  (bind _handle (Variables|Default|GetHandle))
  (bind _keycardtag (Variables|Default|GetKeyCardTag))
  (bind _activegameplaytags (Variables|/Script/HDZMSandbox.SActionComponent|GetActiveGameplayTags _returnvalue))
  (Class|SGamePlayInterface|Interact(Message) (Variables|Default|GetSelectedActor) InstigatorPawn)
  (Utilities|FlowControl|FlipFlop
    (:A
      (Transformation|SetRelativeRotation _handle (Math|Rotator|MakeRotator 0.0 -3e+01 0.0) false false)
      (GameplayTags|AddGameplayTag _activegameplaytags _keycardtag :!class /Script/GameplayTags.BlueprintGameplayTagLibrary))
    (:B
      (Transformation|SetRelativeRotation _handle "30.000000, 0, 0" false false)
      (GameplayTags|RemoveGameplayTag _activegameplaytags _keycardtag :!class /Script/GameplayTags.BlueprintGameplayTagLibrary))))

(fn ConstructionScript)