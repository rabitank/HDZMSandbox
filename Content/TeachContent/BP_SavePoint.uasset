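; BP_SavePoint is an interactable save point actor that writes the world save and lights a fire effect.
; Interact sets IsActiveSave, calls WriteSaveGame on SGameModeBase, prints a confirmation and runs UpdateFire.
; UpdateFire activates the particle system only when IsActiveSave is true.
; OnActorLoaded also runs UpdateFire, so the fire reflects the flag after loading.
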(event Custom|UpdateFire
  (if (Variables|Default|GetbIsActiveSave)
    (Components|Activation|Activate (Variables|Default|GetParticleSystem) false)))

(event EventBeginPlay)

(event Collision|EventActorBeginOverlap
  (params (OtherActor :type Actor%20Object%20Reference)))

(event EventTick
  (params (DeltaSeconds :type Float%20%28single-precision%29)))

(event EventInteract
  (params (InstigatorPawn :type Pawn%20Object%20Reference))
  (Variables|Default|SetbIsActiveSave true)
  (Class|SGameModeBase|WriteSaveGame (.AsSGame%20Mode%20Base (Utilities|Casting|CastToSGameModeBase (Game|GetGameMode))))
  (Development|PrintString "World Saved")
  (CallFunction|UpdateFire))

(event EventOnActorLoaded
  (CallFunction|UpdateFire))

(fn ConstructionScript)