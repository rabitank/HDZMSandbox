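; BP_Blackhole is a black hole projectile that activates a force and destroys physics objects that touch it.
; On spawn, its sphere ignores the instigator when moving, and a short timer then activates the particle effect and force component.
; A second timer destroys the projectile a few seconds later.
; Sphere overlaps destroy the other actor when the overlapped component simulates physics.
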(event OnComponentBeginOverlap(ComSphere)
  (params (OverlappedComponent :type Primitive%20Component%20Object%20Reference) (OtherActor :type Actor%20Object%20Reference) (OtherComp :type Primitive%20Component%20Object%20Reference) (OtherBodyIndex :type Integer) (bFromSweep :type Boolean) (SweepResult :type Hit%20Result%20Structure%20%28by%20ref%29))
  (if (Physics|IsSimulatingPhysics OtherComp "None")
    (Actor|DestroyActor OtherActor)))

(event Custom|ReleaseForce
  (Components|Activation|Activate (Variables|Default|GetComEffectParticle) false)
  (Components|Activation|Activate (Variables|Default|GetComExplodForce) false)
  (Utilities|Time|SetTimerbyEvent (delegate Custom|Destory) 5.0))

(event Custom|Destory
  (Actor|DestroyActor))

(event EventBeginPlay
  (Collision|IgnoreActorwhenMoving (Variables|Default|GetComSphere) (Variables|Default|GetInstigator) true)
  (Utilities|Time|SetTimerbyEvent (delegate Custom|ReleaseForce) 0.2))

(event Collision|EventActorBeginOverlap
  (params (OtherActor :type Actor%20Object%20Reference)))

(event EventTick
  (params (DeltaSeconds :type Float%20%28single-precision%29)))

(fn ConstructionScript)